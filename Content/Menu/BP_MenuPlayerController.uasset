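; Player controller for the main menu that shows the cursor and menu widget and starts hosting or joining of network sessions.
; Hosting passes through to BP_NetworkGameInstance.
; Joining searches for sessions on LAN or online and has the game instance join the first result without checking for an empty list, or disconnect on failure.
; Both actions raise a loading screen above the menu, removed only when the controller is destroyed.
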(event Custom|HostSession
  (params (MaxPlayer :type Integer) (isLan :type Boolean))
  (CallFunction|AddLoadingScreen)
  (Default|HostSession (Variables|Default|GetmyGameInstance) self MaxPlayer isLan))

(event Custom|JoinFirstSession
  (params (isLan :type Boolean))
  (CallFunction|AddLoadingScreen)
  (Development|PrintString "Joining First Sesson" true true "(R=1.000000,G=0.034335,B=0.000000,A=1.000000)" 1e+01)
  (bind _results (|FindSessions self 50 isLan)
    (:OnSuccess
      (Default|JoinSession (Variables|Default|GetmyGameInstance) self (Utilities|Array|Get(acopy) _results)))
    (:OnFailure
      (Default|Disconnect (Variables|Default|GetmyGameInstance) self))))

(event Custom|SetGameInstance
  (bind _asbp_network_game_instance (Utilities|Casting|CastToBP_NetworkGameInstance (Game|GetGameInstance)))
  (Variables|Default|SetmyGameInstance _asbp_network_game_instance))

(event EventBeginPlay
  (CallFunction|SetGameInstance)
  (Variables|Default|SetbShowMouseCursor true)
  (CallFunction|AddMainMenuWdiget))

(event EventDestroyed
  (CallFunction|RemoveLoadingScreen))

(event Custom|AddMainMenuWdiget
  (bind _returnvalue (UserInterface|CreateWidget "/Game/Menu/Widgets/MainMenu.MainMenu_C" self))
  (bind _output_get (Variables|Default|SetMainMenuWidget _returnvalue))
  (UserInterface|Viewport|AddtoPlayerScreen _output_get))

(event Custom|AddLoadingScreen
  (bind _returnvalue (UserInterface|CreateWidget "/Game/Menu/Widgets/LoadingScreen.LoadingScreen_C" self))
  (bind _output_get (Variables|Default|SetLoadingScreenWidget _returnvalue))
  (UserInterface|Viewport|AddtoPlayerScreen _output_get 100))

(event Custom|RemoveLoadingScreen
  (bind _loadingscreenwidget (Variables|Default|GetLoadingScreenWidget)
    (:then
      (Widget|RemovefromParent _loadingscreenwidget)
      (Variables|Default|SetLoadingScreenWidget 0))
    (:else)))

(fn ConstructionScript)