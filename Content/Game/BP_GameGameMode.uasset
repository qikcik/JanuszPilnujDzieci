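; BP_GameGameMode is the game mode that starts a networked match once the expected number of players has joined.
; On BeginPlay it reads the expected player count from BP_NetworkGameInstance.
; Each PostLogin compares that count with the game state's PlayerArray.
; When they match, it waits briefly, then calls StartGame on every player state's owning BP_GamePlayerController.
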(event EventBeginPlay
  (bind _asbp_network_game_instance (Utilities|Casting|CastToBP_NetworkGameInstance (Game|GetGameInstance)))
  (Variables|Default|SetMaxPlayer (Variables|/Game/Blueprints/BP_NetworkGameInstance.BP_NetworkGameInstance_C|GetnumbersOfPlayers _asbp_network_game_instance)))

(event EventPostLogin
  (params (NewPlayer :type Player%20Controller%20Object%20Reference))
  (bind _asbp_game_game_state (Utilities|Casting|CastToBP_GameGameState (Game|GetGameState)))
  (if (== (Variables|Default|GetMaxPlayer) (Utilities|Array|Length (Variables|/Script/Engine.GameStateBase|GetPlayerArray _asbp_game_game_state)))
    (Utilities|FlowControl|Delay 3.0)
    (for _array_element (Variables|/Script/Engine.GameStateBase|GetPlayerArray _asbp_game_game_state)
      (bind _asbp_game_player_controller (Utilities|Casting|CastToBP_GamePlayerController (Components|GetOwner _array_element)))
      (Default|StartGame _asbp_game_player_controller))))

(fn ConstructionScript)