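; BP_GameGameState is a game state that relays match events for pawn hits, counting start and stop, game start and wins through event dispatcher calls.
; Win passes the IsB result to WinMulticast, which fires the win-state dispatcher.
; After a short delay, Win loops over PlayerArray and runs a servertravel console command to the Beach map through each player's controller, stopping if a cast fails.
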(event Custom|PawnHitPawn
  (params (Pawn :type Actor%20Object%20Reference))
  (Default|CallPawnHitPawnForward Pawn))

(event Custom|CountStop
  (Default|CallStopCounting))

(event Custom|CountStart
  (Development|PrintString "asdadasdas")
  (Default|CallStartCounting))

(event Custom|StartGame
  (Default|CallStartGae))

(event Custom|Win
  (params (isB :type Boolean))
  (Development|PrintString "Starting Game" true true "(R=1.000000,G=0.000000,B=0.697727,A=1.000000)" 1e+01)
  (CallFunction|WinMulticast isB)
  (Utilities|FlowControl|Delay 1.0)
  (for _array_element (Variables|Default|GetPlayerArray)
    (bind _asplayer_controller (Utilities|Casting|CastToPlayerController (Components|GetOwner _array_element)))
    (Development|ExecuteConsoleCommand "servertravel Beach" _asplayer_controller)))

(event Custom|WinMulticast
  (params (isB :type Boolean))
  (Default|CallWinState isB))

(event EventBeginPlay)

(event EventTick
  (params (DeltaSeconds :type Float%20%28single-precision%29)))

(fn ConstructionScript)