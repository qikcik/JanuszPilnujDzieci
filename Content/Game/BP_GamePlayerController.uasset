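; Game player controller Blueprint that prints the local player's team ID as debug output when play begins.
; BeginPlay runs the parent logic, then calls BeginPlayLocally, which waits a very short delay before casting the PlayerState to BP_CorePlayerState and printing its TeamId.
; Tick is disabled and the construction script only calls its parent.
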(event Custom|BeginPlayLocally
  (Utilities|FlowControl|Delay 0.01)
  (bind _asbp_core_player_state (Utilities|Casting|CastToBP_CorePlayerState (Variables|Default|GetPlayerState self)))
  (Development|PrintString (Utilities|String|ToString(Integer) (Variables|/Game/Blueprints/BP_CorePlayerState.BP_CorePlayerState_C|GetTeamId _asbp_core_player_state))))

(event EventBeginPlay
  (|CallParentFunction)
  (CallFunction|BeginPlayLocally))

(event EventTick
  (params (DeltaSeconds :type Float%20%28single-precision%29))
  (|CallParentFunction DeltaSeconds) ; This node is disabled and will not be called.\nDrag off pins to build functionality.
)

(fn ConstructionScript
  (|CallParentFunction))