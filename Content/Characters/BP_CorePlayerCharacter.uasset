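; Networked player character that moves, carries and drops objects, and can hit other players with damageable held items.
; It acts as interaction host and interactable: overlaps register candidates, Tick focuses the nearest valid one, and focused characters get a stencil outline.
; Being hit drops the held item, stuns temporarily and notifies the game state.
; OnRep functions drive held mesh, walk speed, movement locks and camera shake.
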(event Custom|uncarring
  (Variables|Default|SetisHolding false))

(event Custom|carring
  (Variables|Default|SetisHolding true))

(event Custom|removeOutline
  (Rendering|SetCustomDepthStencilValue (Variables|Character|GetMesh) 38)
  (Rendering|SetCustomDepthStencilValue (Variables|Default|GetObjectInHand) 38))

(event Custom|AddOutline
  (Rendering|SetCustomDepthStencilValue (Variables|Character|GetMesh) 252)
  (Rendering|SetCustomDepthStencilValue (Variables|Default|GetObjectInHand) 252))

(event Custom|DisconnectSession
  (bind _asbp_network_game_instance (Utilities|Casting|CastToBP_NetworkGameInstance (Game|GetGameInstance)))
  (Default|Disconnect _asbp_network_game_instance (Game|GetPlayerController 0) true))

(event EventBeginPlay
  (CallFunction|RemoveOutline))

(event Collision|EventActorBeginOverlap
  (params (OtherActor :type Actor%20Object%20Reference)))

(event EventTick
  (params (DeltaSeconds :type Float%20%28single-precision%29))
  (CallFunction|UpdateFocus))

(event Custom|Hit
  (Variables|Default|SetisHitted true)
  (if (Variables|Default|GetisHolding)
    (CallFunction|Spawn))
  (Utilities|FlowControl|Delay 3.5)
  (Variables|Default|SetisHitted false))

(event Custom|PlayAnimation
  (params (Duration :type Float%20%28single-precision%29) (animationPlaying :type AnimationStateEnum%20Enum :default "NewEnumerator0"))
  (Variables|Default|SetanimationPlaying animationPlaying)
  (Utilities|FlowControl|Delay Duration)
  (Variables|Default|SetanimationPlaying "NewEnumerator0"))

(event Custom|CameraShake
  (params (Shake :type Camera%20Shake%20Class%20Reference))
  (Camera|PlayWorldCameraShake Shake (Transformation|GetActorLocation) 5.0 9999999.0 0.0))

(event Input|AxisEvents|InputAxismoveForward
  (params (AxisValue :type Float%20%28single-precision%29))
  (Pawn|Input|AddMovementInput (Math|Vector|GetForwardVector (Math|Rotator|MakeRotator 0.0 0.0 (.yaw (Pawn|GetControlRotation :!class /Script/Engine.Pawn)))) AxisValue false))

(event Input|AxisEvents|InputAxismoveRight
  (params (AxisValue :type Float%20%28single-precision%29))
  (Pawn|Input|AddMovementInput (Math|Vector|GetRightVector (Math|Rotator|MakeRotator 0.0 0.0 (.yaw (Pawn|GetControlRotation :!class /Script/Engine.Pawn)))) AxisValue false))

(event Custom|UpdateFocus
  (bind _best (CallFunction|GetBestInteraction))
  (if (not (== _best (Variables|Default|GetFocusedInteractionable)))
    (Utilities|IsValid (Variables|Default|GetFocusedInteractionable)
      (:Is%20Valid
        (Class|Interactionable|LostFocus(Message) (Variables|Default|GetFocusedInteractionable)))
      (:Is%20Not%20Valid
        _))
    (bind _output_get (Variables|Default|SetFocusedInteractionable _best))
    (Class|Interactionable|GetFocus(Message) _output_get self)
    (Development|PrintString "Hello")))

(event Custom|ToInteract
  (params (toInteract :type Actor%20Object%20Reference))
  (Utilities|IsValid toInteract
    (:Is%20Valid
      (bind _can (Class|Interactionable|CanInteract(Message) toInteract self))
      (if _can
        (Class|Interactionable|Interact(Message) toInteract self)))
    (:Is%20Not%20Valid
      (if (.ispickupable (Variables|Default|GetHoldingObject))
        (CallFunction|Spawn)))))

(event Custom|Spawn
  (bind _returnvalue (Transformation|GetActorRotation))
  (bind _objectinhand (Variables|Default|GetObjectInHand))
  (bind _returnvalue_2 (Transformation|GetWorldTransform _objectinhand))
  (bind (_location _rotation _scale) (Math|Transform|BreakTransform _returnvalue_2))
  (bind _returnvalue_3 (Game|SpawnActorfromClass (.actor (Variables|Default|GetHoldingObject)) (Math|Transform|MakeTransform (+ _location (* (Math|Vector|GetForwardVector _returnvalue) 1e+01) (* (Math|Vector|GetUpVector _returnvalue) 20)) _rotation _scale) "AdjustIfPossibleButAlwaysSpawn" 0 0))
  (bind _asgame_object_base (Utilities|Casting|CastToGameObjectBase _returnvalue_3)
    (:then
      (Variables|/Game/objects/GameObjectBase.GameObjectBase_C|SetObjectInfo _asgame_object_base (Variables|Default|GetHoldingObject)))
    (:CastFailed
      _))
  (Variables|Default|SetHoldingObject ""))

(event Custom|SetHoldingObject
  (params (HoldingObject :type Object%20Info%20Struct%20Structure))
  (Variables|Default|SetHoldingObject HoldingObject))

(event EventRegisterInteraction
  (params (Interactor :type Actor%20Object%20Reference))
  (Utilities|DoIam
    (:then
      (bind _returnvalue (Utilities|Array|AddUnique (Variables|Default|GetRegisteredInteractionable) Interactor))
      (Development|PrintString (Utilities|String|ToString(Integer) _returnvalue)))))

(event EventUnregisterInteraction
  (params (interactor :type Actor%20Object%20Reference))
  (Utilities|DoIam
    (:then
      (Utilities|Array|RemoveItem (Variables|Default|GetRegisteredInteractionable) interactor))))

(event Input|ActionEvents|InputActionInteract
  (params (Key :type Key%20Structure))
  (:Pressed
    (CallFunction|ToInteract (Variables|Default|GetFocusedInteractionable))))

(event Input|ActionEvents|InputActionAction2
  (params (Key :type Key%20Structure))
  (:Pressed
    (Variables|Default|SetisHitted true)
    (Pawn|Components|CharacterMovement|SetMovementMode (Variables|Character|GetCharacterMovement) "MOVE_None" 0))
  (:Released
    (Variables|Default|SetisHitted false)
    (Pawn|Components|CharacterMovement|SetMovementMode (Variables|Character|GetCharacterMovement) "MOVE_Walking" 0)))

(event OnComponentBeginOverlap(Capsule)
  (params (OverlappedComponent :type Primitive%20Component%20Object%20Reference) (OtherActor :type Actor%20Object%20Reference) (OtherComp :type Primitive%20Component%20Object%20Reference) (OtherBodyIndex :type Integer) (bFromSweep :type Boolean) (SweepResult :type Hit%20Result%20Structure%20%28by%20ref%29))
  (Class|InteractionHost|RegisterInteraction(Message) OtherActor self))

(event OnComponentEndOverlap(Capsule)
  (params (OverlappedComponent :type Primitive%20Component%20Object%20Reference) (OtherActor :type Actor%20Object%20Reference) (OtherComp :type Primitive%20Component%20Object%20Reference) (OtherBodyIndex :type Integer))
  (Class|InteractionHost|UnregisterInteraction(Message) OtherActor self))

(event EventGetFocus
  (params (interactionHost :type Actor%20Object%20Reference))
  (CallFunction|AddOutline))

(event EventLostFocus
  (CallFunction|RemoveOutline))

(event EventInteract
  (params (InteractionHost :type Actor%20Object%20Reference))
  (Utilities|FlowControl|Sequence
    (:then_0
      (CallFunction|Hit)
      (bind _asbp_core_player_character (Utilities|Casting|CastToBP_CorePlayerCharacter InteractionHost))
      (CallFunction|PlayAnimation _asbp_core_player_character 0.2 "NewEnumerator1"))
    (:then_1
      (bind _asbp_game_game_state (Utilities|Casting|CastToBP_GameGameState (Game|GetGameState)))
      (Default|PawnHitPawn _asbp_game_game_state _asbp_core_player_character))))

(fn ConstructionScript
  (Collision|SetCollisionEnabled (Variables|Default|GetSphere) "NoCollision")
  (Rendering|SetVisibility (Variables|Default|GetObjectInHand) false true))

(fn OnRepIsCarrying)

(fn GetBestInteraction
  (LocalVariables|SetCurrentBestDot 9.223372036854776e+18)
  (LocalVariables|SetCurrentBestIneractionable 0)
  (for _array_element (Variables|Default|GetRegisteredInteractionable)
    (Utilities|IsValid _array_element
      (:Is%20Valid
        (bind _can (Class|Interactionable|CanInteract(Message) _array_element self))
        (if _can
          (if (not (Variables|Default|GetisHitted))
            (bind _center (Class|Interactionable|GetPositionOfCenter(Message) _array_element))
            (if (< (Math|Vector|VectorLength (- _center (Transformation|GetWorldLocation (Variables|Character|GetMesh self)))) (LocalVariables|GetCurrentBestDot))
              (LocalVariables|SetCurrentBestDot (Math|Vector|VectorLength (- _center (Transformation|GetWorldLocation (Variables|Character|GetMesh self)))))
              (LocalVariables|SetCurrentBestIneractionable _array_element)))))))
  (return (LocalVariables|GetCurrentBestIneractionable)))

(fn OnRepHoldingObject
  (bind _holdingobject (Variables|Default|GetHoldingObject))
  (bind _charactermovement (Variables|Character|GetCharacterMovement))
  (bind _sphere (Variables|Default|GetSphere))
  (bind _objectinhand (Variables|Default|GetObjectInHand))
  (if (Utilities|Enum|Equal(Enum) (.type (Variables|Default|GetHoldingObject)) "NewEnumerator1")
    (Variables|Default|SetisHolding false)
    (Variables|/Script/Engine.CharacterMovementComponent|SetMaxWalkSpeed _charactermovement 6e+02)
    (Collision|SetCollisionEnabled _sphere "NoCollision")
    (Rendering|SetVisibility (Variables|Default|GetObjectInHand) false true)
    (else
      (Variables|Default|SetisHolding true)
      (Variables|/Script/Engine.CharacterMovementComponent|SetMaxWalkSpeed _charactermovement 3e+02)
      (Collision|SetCollisionEnabled _sphere "QueryAndPhysics")
      (Components|StaticMesh|SetStaticMesh _objectinhand (.mesh _holdingobject))
      (Transformation|SetRelativeTransform (Variables|Default|GetObjectInHand) (.inhandtransform _holdingobject) false false)
      (Rendering|SetVisibility _objectinhand true true))))

(fn OnRepIsHitted
  (if (Variables|Default|GetisHitted)
    (Pawn|Components|CharacterMovement|SetMovementMode (Variables|Character|GetCharacterMovement) "MOVE_None" 0)
    (Utilities|DoIam
      (:then
        (Camera|PlayWorldCameraShake "/Game/Characters/HittedCameraShake.HittedCameraShake_C" (Transformation|GetActorLocation) 5.0 9999999.0 0.0)))
    (else
      (Pawn|Components|CharacterMovement|SetMovementMode (Variables|Character|GetCharacterMovement) "MOVE_Walking" 0))))

(fn OnRepIsHitting
  (if true
    (Pawn|Components|CharacterMovement|SetMovementMode (Variables|Character|GetCharacterMovement) "MOVE_None" 0)
    (else
      (Pawn|Components|CharacterMovement|SetMovementMode (Variables|Character|GetCharacterMovement) "MOVE_Walking" 0))))

(fn OnRepAnimation)

(fn OnRepAnimationPlaying
  (if (not (Utilities|Enum|Equal(Enum) (Variables|Default|GetanimationPlaying) "NewEnumerator0"))
    (Pawn|Components|CharacterMovement|SetMovementMode (Variables|Character|GetCharacterMovement) "MOVE_None" 0)
    (else
      (Pawn|Components|CharacterMovement|SetMovementMode (Variables|Character|GetCharacterMovement) "MOVE_Walking" 0))))

(fn CanInteract
  (params (InteractionHost :type Actor%20Object%20Reference))
  (if (!= InteractionHost self)
    (bind _asbp_core_player_character (Utilities|Casting|CastToBP_CorePlayerCharacter InteractionHost)
      (:then
        (if (Math|Boolean|ANDBoolean (Variables|BP_CorePlayerCharacter_C|GetisHolding _asbp_core_player_character) (not (Variables|Default|GetisHitted)) (Utilities|Enum|Equal(Enum) (Variables|Default|GetanimationPlaying) "NewEnumerator0"))
          (return (.isdemageble (Variables|BP_CorePlayerCharacter_C|GetHoldingObject _asbp_core_player_character)))
          (else
            _)))
      (:CastFailed
        _))
    (return false)
    (else
      (return false))))

(fn GetPositionOfCenter
  (return "0, 0, 0"))