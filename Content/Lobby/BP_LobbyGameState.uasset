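; Lobby game state that relays team membership and countdown signals between the lobby game mode and listeners.
; It caches BP_LobbyGameMode on BeginPlay and forwards player register and unregister calls, with their team flag, to it.
; Multicast-named events fire calls for team updates and countdown start or stop, and a getter supplies a fixed countdown length.
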(event EventBeginPlay
  (bind _asbp_lobby_game_mode (Utilities|Casting|CastToBP_LobbyGameMode (Game|GetGameMode)))
  (Variables|Default|SetmyGameMode _asbp_lobby_game_mode))

(event Custom|UnregisterPlayer
  (params (is%20B :type Boolean) (PlayerContrlloer :type BP%20Lobby%20Player%20Controller%20Object%20Reference%20%28by%20ref%29))
  (Default|UnregisterPlayer (Variables|Default|GetmyGameMode) is%20B PlayerContrlloer))

(event Custom|StartCountingMulticast
  (Default|CallStartCounting))

(event Custom|Register%20Player
  (params (isB :type Boolean) (PlayerController :type BP%20Lobby%20Player%20Controller%20Object%20Reference))
  (Default|RegisterPlayer (Variables|Default|GetmyGameMode) isB PlayerController))

(event Custom|StopCountingMulticast
  (Default|CallStopCounting))

(event Custom|UpdateTeamMulticast
  (params (Actual%20Team%20A :type Integer) (Actual%20Team%20B :type Integer) (Max%20Players :type Integer))
  (Default|CallUpdateTeams Actual%20Team%20A Actual%20Team%20B Max%20Players))

(fn ConstructionScript)

(fn GetCountingTime
  (return 5))