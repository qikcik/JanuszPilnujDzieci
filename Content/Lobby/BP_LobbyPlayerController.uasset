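; Lobby player controller that shows and hides a countdown screen for the player before the start.
; On BeginPlay it caches BP_LobbyGameState and binds to its start-counting and stop-counting events.
; Starting creates a WBP_LobbyCounting widget seeded with the game state's counting time and adds it to the player's screen; stopping removes and clears it.
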(event EventBeginPlay
  (bind _asbp_lobby_game_state (Utilities|Casting|CastToBP_LobbyGameState (Game|GetGameState)))
  (Variables|Default|SetmyGameState _asbp_lobby_game_state)
  (CallFunction|CountingBeginPlay))

(event Custom|StartCountingToStart
  (bind _seconds (Default|GetCountingTime (Variables|Default|GetmyGameState)))
  (bind _returnvalue (UserInterface|CreateWidget "/Game/Lobby/WBP_LobbyCounting.WBP_LobbyCounting_C" self _seconds))
  (bind _output_get (Variables|Default|SetCountingScreen _returnvalue))
  (UserInterface|Viewport|AddtoPlayerScreen _output_get))

(event Custom|StopCountingToStart
  (bind _countingscreen (Variables|Default|GetCountingScreen)
    (:then
      (Widget|RemovefromParent _countingscreen)
      (Variables|Default|SetCountingScreen 0))
    (:else)))

(event Custom|CountingBeginPlay
  (Utilities|FlowControl|Sequence
    (:then_0
      (EventDispatchers|BindEventtoStartCounting (Variables|Default|GetmyGameState) (delegate Custom|StartCountingToStart)))
    (:then_1
      (EventDispatchers|BindEventtoStopCounting (Variables|Default|GetmyGameState) (delegate Custom|StopCountingToStart)))))

(fn ConstructionScript
  (|CallParentFunction))