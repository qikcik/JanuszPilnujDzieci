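; BP_CorePlayerState is a player state that preserves a player's team flag (IsB) through the game instance.
; On Destroyed it writes the save data into BP_NetworkGameInstance's PlayerStateSave map, keyed by the owning PlayerController's controller ID.
; On BeginPlay it looks up that key and, if found, restores IsB from the saved TeamId.
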(event EventBeginPlay
  (CallFunction|Load))

(event EventDestroyed
  (CallFunction|Save))

(event Custom|Save
  (bind _asplayer_controller (Utilities|Casting|CastToPlayerController (Components|GetOwner self)))
  (bind _asbp_network_game_instance (Utilities|Casting|CastToBP_NetworkGameInstance (Game|GetGameInstance)))
  (bind _save (CallFunction|SaveData))
  (Utilities|Map|Add (Variables|/Game/Blueprints/BP_NetworkGameInstance.BP_NetworkGameInstance_C|GetPlayerStateSave _asbp_network_game_instance) (Class|GameplayStatics|GetPlayerControllerID _asplayer_controller) _save))

(event Custom|Load
  (bind _asplayer_controller (Utilities|Casting|CastToPlayerController (Components|GetOwner self)))
  (bind _asbp_network_game_instance (Utilities|Casting|CastToBP_NetworkGameInstance (Game|GetGameInstance)))
  (if (.ReturnValue (Utilities|Map|Find (Variables|/Game/Blueprints/BP_NetworkGameInstance.BP_NetworkGameInstance_C|GetPlayerStateSave _asbp_network_game_instance) (Class|GameplayStatics|GetPlayerControllerID _asplayer_controller)))
    (CallFunction|LoadData (.Value (Utilities|Map|Find (Variables|/Game/Blueprints/BP_NetworkGameInstance.BP_NetworkGameInstance_C|GetPlayerStateSave _asbp_network_game_instance) (Class|GameplayStatics|GetPlayerControllerID _asplayer_controller))))))

(fn ConstructionScript)

(fn SaveData
  (return (Utilities|Struct|MakeCorePlayerData_Structure (Variables|Default|GetisB))))

(fn LoadData
  (params (Load :type Core%20Player%20Data%20Structure%20Structure))
  (Variables|Default|SetisB (.teamid Load)))