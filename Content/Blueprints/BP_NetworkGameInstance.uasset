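; BP_NetworkGameInstance is a game instance Blueprint that manages multiplayer session hosting, joining and disconnecting.
; Hosting creates a session with a player limit and LAN option, then opens the Lobby level as a listen server on success.
; Joining uses a supplied session search result, while disconnecting destroys the session and returns to the Menu level whether that succeeds or fails.
; Travel and network errors print their failure type on screen in red.
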(event Custom|HostSession
  (params (PlayerController :type Player%20Controller%20Object%20Reference) (MaxPlayer :type Integer) (isLan :type Boolean))
  ;[1 1 1] Launch Lobby witch Host Setting
  (|Session PlayerController MaxPlayer isLan
    (:OnSuccess
      (Game|OpenLevel(byName) "Lobby" true "listen"))))

(event Custom|Disconnect
  (params (PlayerController :type Player%20Controller%20Object%20Reference))
  (|DestroySession PlayerController
    (:OnSuccess
      _)
    (:OnFailure
      _))
  (Game|OpenLevel(byName) "Menu"))

(event Custom|JoinSession
  (params (PlayerController :type Player%20Controller%20Object%20Reference) (Session :type Blueprint%20Session%20Result%20Structure))
  ;[1 1 1] Join Session
  (|JoinSession PlayerController Session))

(event EventHandleNetworkError
  (params (FailureType :type ENetworkFailure%20Enum :default "NetDriverAlreadyExists") (bIsServer :type Boolean))
  (Development|PrintString (Utilities|String|EnumtoString FailureType) true true "(R=1.000000,G=0.000000,B=0.025802,A=1.000000)" 1e+01))

(event EventHandleTravelError
  (params (FailureType :type ETravelFailure%20Enum :default "NoLevel"))
  (Development|PrintString (Utilities|String|EnumtoString FailureType) true true "(R=1.000000,G=0.000000,B=0.025802,A=1.000000)" 1e+01))