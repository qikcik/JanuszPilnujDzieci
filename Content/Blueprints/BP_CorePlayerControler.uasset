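; BP_CorePlayerControler is a player controller that shows countdown and win-state UI in response to game state events.
; On BeginPlay it casts the game state to BP_GameGameState and binds to its start counting, stop counting and win state dispatchers.
; Start creates and stores a Counting widget on the player screen, stop removes and clears it, and win state adds a WinState widget carrying the IsB flag.
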(event Custom|CounterStop
  (Utilities|IsValid (Variables|Default|Getco)
    (:Is%20Valid
      (Widget|RemovefromParent (Variables|Default|Getco))
      (Variables|Default|Setco 0))))

(event Custom|CounterStart
  (bind _returnvalue (UserInterface|CreateWidget "/Game/Counting.Counting_C"))
  (bind _output_get (Variables|Default|Setco _returnvalue))
  (UserInterface|Viewport|AddtoPlayerScreen _output_get))

(event Custom|registerCounter
  (bind _asbp_game_game_state (Utilities|Casting|CastToBP_GameGameState (Game|GetGameState)))
  (EventDispatchers|AssignStartCounting _asbp_game_game_state (delegate Custom|CounterStart))
  (EventDispatchers|BindEventtoStopCounting _asbp_game_game_state (delegate Custom|CounterStop))
  (EventDispatchers|BindEventtoWinState _asbp_game_game_state (delegate Custom|CustomEvent_0)))

(event Custom|CustomEvent_0
  (params (isB :type Boolean))
  (bind _returnvalue (UserInterface|CreateWidget "/Game/WinState.WinState_C" 0 isB))
  (UserInterface|Viewport|AddtoPlayerScreen _returnvalue))

(event EventBeginPlay
  (CallFunction|RegisterCounter))

(fn ConstructionScript)